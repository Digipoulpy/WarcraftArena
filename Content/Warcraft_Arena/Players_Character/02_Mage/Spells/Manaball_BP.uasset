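; Mage Manaball spell actor that deals random damage to the first overlapping actor tagged Enemy.
; On spawn, a short looping timer leaves scaled-down wave particle effects at the Arrow's location for two seconds.
; The collision sphere switches to query-only after a brief delay; a hit applies damage credited to player 0, spawns an impact wave and destroys the ball shortly after.
; Without a hit, it destroys itself after about ten seconds.
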(event `Waves`
  ;[1 1 1] Wave Spawn
  (`KismetSystemLibrary.K2_SetTimer` null "WaveSpawner" 0.1 true)
  (`KismetSystemLibrary.Delay` 2.0)
  (`KismetSystemLibrary.K2_ClearTimer` null "WaveSpawner"))

(event `self.ReceiveBeginPlay`
  (`self.Waves`)
  (`KismetSystemLibrary.Delay` 0.1)
  (`PrimitiveComponent.SetCollisionEnabled` (`self.Collisionball`) "QueryOnly")
  (`KismetSystemLibrary.Delay` 10.0)
  (`self.K2_DestroyActor`))

(event `self.Collisionball.OnComponentBeginOverlap`
  (params (OverlappedComponent :type "PrimitiveComponent Object Reference") (OtherActor :type "Actor Object Reference") (OtherComp :type "PrimitiveComponent Object Reference") (OtherBodyIndex :type Integer) (bFromSweep :type Boolean) (SweepResult :type "HitResult Structure (by ref)"))
  (bind _output_get (set `self.OtherActor` OtherActor))
  (if (`self.ActorHasTag` _output_get "Enemy")
    (`GameplayStatics.ApplyDamage` (`self.OtherActor`) (`KismetMathLibrary.RandomFloatInRange` 10.0 30.0) (`GameplayStatics.GetPlayerController` 0))
    (`GameplayStatics.SpawnEmitterAtLocation` "/Game/WarcraftArena/Particles/Warrior/P_WaveSprite.P_WaveSprite" (`SceneComponent.K2_GetComponentLocation` (`self.Collisionball`)))
    (`KismetSystemLibrary.Delay` 0.05)
    (`self.K2_DestroyActor`)))

(fn `UserConstructionScript`)

(fn `WaveSpawner`
  (bind _returnvalue (`GameplayStatics.SpawnEmitterAtLocation` "/Game/WarcraftArena/Particles/Warrior/P_WaveSprite.P_WaveSprite" (`SceneComponent.K2_GetComponentLocation` (`self.Arrow`))))
  (`SceneComponent.SetWorldScale3D` _returnvalue (0.5 0.5 0.5)))