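; Bagou_BP is the Blueprint for Bagou, a neutral boss in Warcraft Arena, and handles setup of its elite HUD.
; On BeginPlay it binds to the BagouBoss and Letsgo events.
; The first fills HP, then creates a HUD_Elite widget seeded with health, energy as mana, name and a portrait texture.
; The second adds that prepared widget to the viewport, keeping creation separate from display.
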(event `self.ReceiveBeginPlay`
  (add `self.BagouBoss` (delegate `InitializeBagou`))
  (add `self.Letsgo` (delegate `TimeToGo`)))

(event `InitializeBagou`
  (bind _maxhp (`self.MaxHp`))
  (set `self.HP` _maxhp)
  (bind _returnvalue (`|CreateWidget` "/Game/Warcraft_Arena/UI/Characters/HUD_Elite.HUD_Elite_C"))
  (set `/Game/Warcraft_Arena/UI/Characters/HUD_Elite.MaxHealth` _maxhp _returnvalue)
  (set `/Game/Warcraft_Arena/UI/Characters/HUD_Elite.Health` (`self.HP`) _returnvalue)
  (set `/Game/Warcraft_Arena/UI/Characters/HUD_Elite.MaxMana` (`self.MaxEnergy`) _returnvalue)
  (set `/Game/Warcraft_Arena/UI/Characters/HUD_Elite.Mana` (`self.Energy`) _returnvalue)
  (set `/Game/Warcraft_Arena/UI/Characters/HUD_Elite.Name` (`self.Name`) _returnvalue)
  (`Image.SetBrushFromTexture` (`/Game/Warcraft_Arena/UI/Characters/HUD_Elite.Portrait` _returnvalue) "/Game/Warcraft_Arena/UI/Textures/Backgrounds/AdventureMapParchmentTile.AdventureMapParchmentTile" false))

(event `TimeToGo`
  (`UserWidget.AddToViewport` (stale `InitializeBagou` _returnvalue) 0))

(fn `UserConstructionScript`)