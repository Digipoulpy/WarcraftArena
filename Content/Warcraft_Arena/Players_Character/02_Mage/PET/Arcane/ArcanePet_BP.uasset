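; Mage's Arcane pet character that follows the player or an Enemy-tagged actor and expires as its health drains each second.
; A delayed Seeker loop re-issues AI MoveTo on the target while a timer checks distance, calling Heal near the player or Attack otherwise.
; Heal and Attack only handle montage and state; left-arm overlap, toggled by collision events, deals random damage to enemies.
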(event `self.ReceiveBeginPlay`
  ;[1 1 1] Begin
  (`KismetSystemLibrary.Delay` 0.2)
  (set `self.Target` (`GameplayStatics.GetPlayerCharacter` 0))
  (`self.Seeker`)
  (`KismetSystemLibrary.K2_SetTimer` null "DistanceCheck" 0.1 true)
  (`self.Initialize`))

(event `Initialize`
  ;[1 1 1] Initialize
  (set `self.Health` 100.0)
  (`KismetSystemLibrary.K2_SetTimer` null "Life" 1.0 true))

(event `Kill`
  ;[1 1 1] Kill
  (`/Engine/EditorBlueprintResources/StandardMacros.DoOnce` false
    (:`Completed`
      (bind _returnvalue (`self.PlayAnimMontage` null))
      (`KismetSystemLibrary.Delay` _returnvalue)
      (`self.K2_DestroyActor`))))

(event `Seeker`
  ;[1 1 1] Seeker
  (if (`self.Attacking`)
    (`MovementComponent.StopMovementImmediately` (`self.CharacterMovement`))
    (else
      (`self.Chase`
        (:`Out`
          (`KismetSystemLibrary.Delay` 0.2)
          (`self.Seeker`))))))

(event `Attack`
  ;[1 1 1] Attack Or Heal
  (if (`self.Attacking`)
    (set `self.Attacking` true)
    (`self.PlayAnimMontage` null)))

(event `Heal`
  ;[1 1 1] Attack Or Heal
  (if (`self.Attacking`)
    (set `self.Attacking` true)
    (`self.PlayAnimMontage` null)))

(event `Reset`
  ;[1 1 1] Reset
  (set `self.Attacking` false)
  (`self.Seeker`))

(event `Follow Player`
  ;[1 1 1] Set Player as Target
  (set `self.Target` (`GameplayStatics.GetPlayerCharacter` 0)))

(event `LeftCollision`
  ;[1 1 1] LedtArm Collision
  (`PrimitiveComponent.SetCollisionEnabled` (`self.LeftArm`) "QueryOnly"))

(event `Follow Boss`
  ;[1 1 1] Set Enemy as Target
  (bind _outactors (`GameplayStatics.GetAllActorsOfClass` "/Script/Engine.Character"))
  (for _array_element _outactors
    (if (`self.ActorHasTag` _array_element "Enemy")
      (set `self.Target` _array_element))))

(event `DisableLeftCollision`
  ;[1 1 1] LedtArm Collision
  (`PrimitiveComponent.SetCollisionEnabled` (`self.LeftArm`) "NoCollision"))

(event `self.LeftArm.OnComponentBeginOverlap`
  (params (OverlappedComponent :type "PrimitiveComponent Object Reference") (OtherActor :type "Actor Object Reference") (OtherComp :type "PrimitiveComponent Object Reference") (OtherBodyIndex :type Integer) (bFromSweep :type Boolean) (SweepResult :type "HitResult Structure (by ref)"))
  ;[1 1 1] Left Arm Overlap
  (if (`self.ActorHasTag` OtherActor "Enemy")
    (`GameplayStatics.ApplyDamage` OtherActor (`KismetMathLibrary.RandomFloatInRange` 20.0 30.0) (`GameplayStatics.GetPlayerController` 0))))

(fn `DistanceCheck`
  (if (`self.Attacking`)
    _
    (elif (<= (`KismetMathLibrary.VSize` (- (`self.K2_GetActorLocation`) (`self.K2_GetActorLocation` (`self.Target`)))) 300.0)
      (if (== (`self.Target`) (`GameplayStatics.GetPlayerCharacter` 0))
        (`self.Heal`)
        (else
          (`self.Attack`))))))

(fn `Life`
  (bind _output_get (set `self.Health` (`KismetMathLibrary.FClamp` (- (`self.Health`) 1.0) 0.0 100.0)))
  (if (<= _output_get 0.0)
    (`self.Kill`)))

(fn `UserConstructionScript`)